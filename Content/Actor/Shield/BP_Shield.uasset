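; BP_Shield is a shield actor made of four mesh parts that breaks apart piece by piece as it takes damage.
; When HealthComponent reports a loss of at least HpPerPart since the last break, one random active part is hidden and loses collision.
; Each health change removes at most one part, however large the drop.
; ShieldReset restores health, all parts and the damage threshold.
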(event `self.ReceiveBeginPlay`
  (set `self.ShieldPartsArray` (`|MakeArray` (`self.ShieldMesh0`) (`self.ShieldMesh1`) (`self.ShieldMesh2`) (`self.ShieldMesh3`)))
  (bind _returnvalue (`HealthComponent.GetMaxHealth` (`self.HealthComponent`)))
  (set `self.LastHpOnPartDestruction` (`KismetMathLibrary.FTrunc` _returnvalue))
  (`KismetArrayLibrary.Array_Append` (`self.ActivtePartsArray`) (`self.ShieldPartsArray`)))

(event `self.HealthComponent.OnHealthChange`
  (params (CurrentHealth :type Integer) (MaxHealth :type Integer))
  (if (>= (- (`self.LastHpOnPartDestruction`) CurrentHealth) (`self.HpPerPart`))
    (bind _shieldpart (`self.GetRandomPart` (`self.ActivtePartsArray`)))
    (`KismetArrayLibrary.Array_RemoveItem` (`self.ActivtePartsArray`) _shieldpart)
    (`self.SetState` true _shieldpart)
    (set `self.LastHpOnPartDestruction` CurrentHealth)))

(event `self.ShieldReset`
  (bind _activtepartsarray (`self.ActivtePartsArray`))
  (`HealthComponent.ResetHp` (`self.HealthComponent`))
  (`KismetArrayLibrary.Array_Clear` _activtepartsarray)
  (`KismetArrayLibrary.Array_Append` _activtepartsarray (`self.ShieldPartsArray`))
  (for _array_element (`self.ShieldPartsArray`)
    (`self.SetState` false _array_element)
    (bind _returnvalue (`HealthComponent.GetMaxHealth` (`self.HealthComponent`)))
    (set `self.LastHpOnPartDestruction` (`KismetMathLibrary.FTrunc` _returnvalue))))

(fn `GetRandomPart`
  (params (ShieldPartArray :type "Array of StaticMeshComponent Object Reference"))
  (returns (ShieldPart :type "StaticMeshComponent Object Reference"))
  (return (`|GetArrayItem` ShieldPartArray (`KismetMathLibrary.RandomIntegerInRange` 0 (- (`KismetArrayLibrary.Array_Length` ShieldPartArray) 1)))))

(fn `SetState`
  (params (bIsDead :type Boolean) (ShieldPartMesh :type "StaticMeshComponent Object Reference"))
  (`PrimitiveComponent.SetCollisionEnabled` ShieldPartMesh (select `bool` bIsDead :`false` "QueryAndPhysics" :`true` "NoCollision" :!type "ECollisionEnabled Enum"))
  (`SceneComponent.SetVisibility` ShieldPartMesh (not bIsDead) true))

(fn `UserConstructionScript`)