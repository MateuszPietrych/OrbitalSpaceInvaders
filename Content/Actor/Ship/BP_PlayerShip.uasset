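; BP_PlayerShip is the player ship Blueprint, extending a parent class that provides a ship death event.
; On BeginPlay it binds to that death event and, when it fires, hides BaseSceneComponent and all of its children.
; The construction script only calls the parent version, and the overlap and tick events are disabled stubs.
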(event `self.ReceiveBeginPlay`
  (`parent.ReceiveBeginPlay`)
  (add `self.OnShipDeath` (delegate `OnShipDeath_Event`)))

(event `OnShipDeath_Event` :!signature `self.OnShipDeath`
  (params (DeadShip :type "OrbitalShip Object Reference"))
  (`SceneComponent.SetVisibility` (`self.BaseSceneComponent`) false true))

(fn `UserConstructionScript`
  (`parent.UserConstructionScript`))