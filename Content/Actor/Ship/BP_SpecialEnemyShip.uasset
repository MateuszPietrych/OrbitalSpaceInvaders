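; BP_SpecialEnemyShip is a child ship Blueprint for a special enemy ship variant.
; On BeginPlay, after the parent logic, it smoothly changes its radius to zero and sets its speed to the MaxSpeed from ShipData.
; Tick and construction only call the parent, and the overlap event is disabled, so all other behavior is inherited.
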(event `self.ReceiveBeginPlay`
  (`parent.ReceiveBeginPlay`)
  (`self.ChangeRadiusSmooth` 0.0)
  (`self.ChangeSpeed` (`OrbitalShipDataAsset.MaxSpeed` (`self.ShipData`))))

(event `self.ReceiveTick`
  (params (DeltaSeconds :type "Float (single-precision)"))
  (`parent.ReceiveTick` DeltaSeconds))

(fn `UserConstructionScript`
  (`parent.UserConstructionScript`))