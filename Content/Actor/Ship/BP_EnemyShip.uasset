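; BP_EnemyShip is an enemy ship that deals ram damage on contact and is destroyed in the process.
; At BeginPlay it sets RotatingMovement's yaw rate from ShipData.MaxSpeed and binds OnShipDeath to destroy the actor.
; When CollisionSphereForDirect overlaps a Combat interface implementer, it sends a Direct damage context using ShipData.ShipDamage, then destroys itself.
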(event `self.ReceiveBeginPlay`
  (set `RotatingMovementComponent.RotationRate` (`KismetMathLibrary.MakeRotator` 0.0 0.0 (`OrbitalShipDataAsset.MaxSpeed` (`self.ShipData`))) (`self.RotatingMovement`))
  (add `self.OnShipDeath` (delegate `OnShipDeath_Event`)))

(event `OnShipDeath_Event` :!signature `self.OnShipDeath`
  (params (DeadShip :type "OrbitalShip Object Reference"))
  (`self.K2_DestroyActor`))

(event `self.CollisionSphereForDirect.OnComponentBeginOverlap`
  (params (OverlappedComponent :type "PrimitiveComponent Object Reference") (OtherActor :type "Actor Object Reference") (OtherComp :type "PrimitiveComponent Object Reference") (OtherBodyIndex :type Integer) (bFromSweep :type Boolean) (SweepResult :type "HitResult Structure (by ref)"))
  (if (`KismetSystemLibrary.DoesImplementInterface` OtherActor "/Script/ByteSpaceInvaders.Combat")
    (bind _ascombat (cast `Combat` OtherActor))
    (`Combat.TakeDamage` _ascombat (make `DamageContext` (`OrbitalShipDataAsset.ShipDamage` (`self.ShipData`)) "Direct"))
    (`self.K2_DestroyActor`)))

(fn `UserConstructionScript`)