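; BP_Earth is the Earth actor in the Orbit folder, a damageable body whose health is held in a HealthComponent.
; InitializeEarth seeds that component with its own max health.
; TakeDamage forwards the damage value to the component only for Direct damage, so Projectile hits are ignored.
; GetDamage returns zero, so Earth reports no damage of its own.
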(event `self.ReceiveBeginPlay`)

(event `self.TakeDamage`
  (params (DamageContext :type "DamageContext Structure"))
  (bind (_damagevalue _damagetype) (break `DamageContext` DamageContext))
  (if (select `EDamageType` _damagetype :`Direct` true)
    (`HealthComponent.ApplyDamage` (`self.HealthComponent`) _damagevalue)))

(fn `GetDamage`
  (returns (ReturnValue :type "Float (single-precision)"))
  (return 0.0))

(fn `InitializeEarth`
  (bind _healthcomponent (`self.HealthComponent`))
  (bind _returnvalue (`HealthComponent.GetMaxHealth` _healthcomponent))
  (`HealthComponent.InitializeHealthComponent` _healthcomponent _returnvalue))

(fn `UserConstructionScript`)