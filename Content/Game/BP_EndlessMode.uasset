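; BP_EndlessMode is the endless-mode Blueprint, which advances the game by a level each time a new round starts.
; Both the GameReset_Event event and the StartNewGame function increment Level, then call InitalizeSpawner to set up the spawner.
; BeginPlay and the construction script only call their parent versions, and Tick is disabled.
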(event `self.ReceiveBeginPlay`
  (`parent.ReceiveBeginPlay`))

(event `GameReset_Event`
  (set `self.Level` (+ (`self.Level`) 1))
  (`self.InitalizeSpawner`))

(fn `StartNewGame`
  (set `self.Level` (+ (`self.Level`) 1))
  (`self.InitalizeSpawner`))

(fn `UserConstructionScript`
  (`parent.UserConstructionScript`))