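; Game mode for Bye Space Invaders that sets up the orbit chain and starts enemy spawning on BeginPlay.
; It gathers all Orbit actors, sorts them by descending radius, links them as a linked list and sets the largest as first orbit.
; Sorting uses a radius-keyed map, so orbits sharing a radius collapse into one entry.
; It then tells the level's Spawner to spawn the starting orbital ships.
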(event `self.ReceiveBeginPlay`
  (`|ExecutionSequence`
    (:`then_0`
      ;[1 1 1] Create Linked List From Orbits
      (bind _outactors (`GameplayStatics.GetAllActorsOfClass` "/Script/ByteSpaceInvaders.Orbit"))
      (bind _outorbitlist (`self.SortOrbitListByRadius` _outactors "Descending"))
      (`self.MakeOrbitLinkedList` _outorbitlist)
      (`self.SetFirstOrbit` (`|GetArrayItem` _outorbitlist)))
    (:`then_1`
      ;[1 1 1] Spawn Enemies
      (bind _returnvalue (`GameplayStatics.GetActorOfClass` "/Script/ByteSpaceInvaders.Spawner"))
      (`Spawner.SpawnStartObritalShips` _returnvalue))))

(fn `MakeOrbitLinkedList`
  (params (SortedOrbitList :type "Array of Orbit Object Reference"))
  (for (_array_element _array_index) SortedOrbitList
    (bind _returnvalue (+ _array_index 1))
    (if (< _returnvalue (`KismetArrayLibrary.Array_Length` SortedOrbitList))
      (bind _output (`|GetArrayItem` SortedOrbitList _returnvalue))
      (`LinkedListElement.SetNextElement` _output _output)
      (`LinkedListElement.SetNextElement` _array_element _output))))

(fn `SortOrbitListByRadius`
  (params (InOrbitList :type "Array of Orbit Object Reference") (SortOrder :type "EArraySortOrder Enum" :default "Ascending"))
  (returns (OutOrbitList :type "Array of Orbit Object Reference"))
  (locals (OrbitMap :type "Map of Float (double-precision) to Orbit Object Reference") (FinalArray :type "Array of Orbit Object Reference"))
  (for _array_element InOrbitList
    (bind _returnvalue (`Orbit.GetRadius` _array_element))
    (`BlueprintMapLibrary.Map_Add` (`local.OrbitMap`) _returnvalue _array_element))
  (bind _keys (`BlueprintMapLibrary.Map_Keys` (`local.OrbitMap`)))
  (`KismetArrayLibrary.SortFloatArray` _keys true SortOrder)
  (for _array_element_2 _keys
    (bind (_value _returnvalue_2) (`BlueprintMapLibrary.Map_Find` (`local.OrbitMap`) _array_element_2))
    (if _returnvalue_2
      (`KismetArrayLibrary.Array_Add` (`local.FinalArray`) _value)))
  (return (`local.FinalArray`)))

(fn `UserConstructionScript`)